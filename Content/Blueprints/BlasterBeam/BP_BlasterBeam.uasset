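; BP_BlasterBeam is a blaster beam actor that bursts and disappears when it hits something.
; On BeginPlay it binds the BeamMesh component hit event, whose handler spawns the NS_BeamBurst effect at the impact point, oriented along the surface normal, then destroys the actor.
; The graph applies no damage or movement; Tick is empty, and the leftover offset and debug print nodes never run.
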(event `self.ReceiveBeginPlay`
  (add `PrimitiveComponent.OnComponentHit` (`self.BeamMesh`) (delegate `OnComponentHit_Event`)))

(event `OnComponentHit_Event`
  (params (HitComponent :type "PrimitiveComponent Object Reference") (OtherActor :type "Actor Object Reference") (OtherComp :type "PrimitiveComponent Object Reference") (NormalImpulse :type "Vector Structure") (Hit :type "HitResult Structure (by ref)"))
  (bind (_bblockinghit _binitialoverlap _time _distance _location _impactpoint _normal) (`GameplayStatics.BreakHitResult` Hit))
  (`NiagaraFunctionLibrary.SpawnSystemAtLocation` "/Game/Assets/FX/NS_BeamBurst.NS_BeamBurst" _impactpoint (`KismetMathLibrary.MakeRotFromX` _normal))
  (`self.K2_DestroyActor`))

(event `self.ReceiveTick`
  (params (DeltaSeconds :type "Float (single-precision)")))

(fn `UserConstructionScript`)