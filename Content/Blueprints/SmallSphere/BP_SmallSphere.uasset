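; BP_SmallSphere is a short-lived sphere actor that tumbles through the world and vanishes on contact with a Pawn.
; Timelines scale the mesh on spawn and again on wink-out, which a lifetime timer or Pawn overlap triggers once before the actor is destroyed.
; Tick moves it along its forward vector without sweeping and applies a scaled random spin, so its heading keeps changing.
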(event `self.ReceiveBeginPlay`
  (`self.WinkIn`)
  (`self.InitializeDeltaRotation`)
  ;[1 0.2335 0.1838] StartWinkOutTimeline
  (`KismetSystemLibrary.K2_SetTimerDelegate` (delegate `WinkOut`) (`self.LifeTime`))
  (add `PrimitiveComponent.OnComponentBeginOverlap` (`self.SphereVolume`) (delegate `OnSphereOverlap`)))

(event `OnSphereOverlap`
  (params (OverlappedComponent :type "PrimitiveComponent Object Reference") (OtherActor :type "Actor Object Reference") (OtherComp :type "PrimitiveComponent Object Reference") (OtherBodyIndex :type Integer) (bFromSweep :type Boolean) (SweepResult :type "HitResult Structure (by ref)"))
  (if (`GameplayStatics.ObjectIsA` OtherActor "/Script/Engine.Pawn")
    (`self.WinkOut`)))

(event `WinkOut`
  ;[1 0.2335 0.1838] StartWinkOutTimeline
  (if (not (`self.IsWrinking`))
    (set `self.IsWrinking` true)
    (bind (_direction _scale) (`Timeline|WinkOutTimeline`)
      (:`Update`
        (`self.ScaleSphere` _scale))
      (:`Finished`
        (`self.K2_DestroyActor`)))))

(event `WinkIn`
  ;[1 0.2335 0.1838] Wink into Existence
  (bind (_direction _scale) (`Timeline|WinkInTimeLine`)
    (:`Update`
      (`SceneComponent.SetWorldScale3D` (`self.SphereMesh`) _scale))))

(event `self.ReceiveTick`
  (params (DeltaSeconds :type "Float (single-precision)"))
  ;[0.5069 1 0.7093] Update Location and Rotation
  (`self.UpdateLocation` DeltaSeconds)
  (`self.UpdateRotation` DeltaSeconds))

(fn `InitializeDeltaRotation`
  (set `self.DeltaRotation` (* (`KismetMathLibrary.RandomRotator` false) (`self.RotationScaleFactor`))))

(fn `ScaleSphere`
  (params (Scale :type "Float (single-precision)"))
  (`SceneComponent.SetWorldScale3D` (`self.SphereMesh`) (`KismetMathLibrary.MakeVector` Scale Scale Scale)))

(fn `UpdateLocation`
  (params (A :type "Float (double-precision)"))
  (`self.K2_AddActorWorldOffset` (* (`self.GetActorForwardVector`) (* A (`self.Speed`)))))

(fn `UpdateRotation`
  (params (B :type "Float (single-precision)"))
  (`self.K2_AddActorWorldRotation` (* (`self.DeltaRotation`) B)))

(fn `UserConstructionScript`)