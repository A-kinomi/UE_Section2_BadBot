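; BP_Pawn is the player pawn that takes damage from blaster beams and shows its health on screen.
; On BeginPlay it creates the UMG_PlayerInfo widget and sets starting HP.
; When a BP_BlasterBeam overlaps its Box, it subtracts the beam's damage, updates the widget, prints the damage and destroys the beam.
; The game quits once HP drops below zero.
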(event `self.ReceiveBeginPlay`
  (bind _returnvalue (`|CreateWidget` "/Game/Assets/UMG/UMG_PlayerInfo.UMG_PlayerInfo_C"))
  (bind _output_get (set `self.UMG_PlayerInfo` _returnvalue))
  (`UserWidget.AddToViewport` _output_get 0)
  (bind _output_get_2 (set `self.HP` 100))
  (`/Game/Assets/UMG/UMG_PlayerInfo.ChangeHP` (`self.UMG_PlayerInfo`) _output_get_2))

(event `self.Box.OnComponentBeginOverlap`
  (params (OverlappedComponent :type "PrimitiveComponent Object Reference") (OtherActor :type "Actor Object Reference") (OtherComp :type "PrimitiveComponent Object Reference") (OtherBodyIndex :type Integer) (bFromSweep :type Boolean) (SweepResult :type "HitResult Structure (by ref)"))
  (bind _asbp_blaster_beam (cast `/Game/Blueprints/BlasterBeam/BP_BlasterBeam` OtherActor))
  (bind _damege (`/Game/Blueprints/BlasterBeam/BP_BlasterBeam.Damege` _asbp_blaster_beam))
  (bind _output_get (set `self.HP` (- (`self.HP`) _damege)))
  (`/Game/Assets/UMG/UMG_PlayerInfo.ChangeHP` (`self.UMG_PlayerInfo`) _output_get)
  (`KismetSystemLibrary.PrintString` (`KismetStringLibrary.Conv_IntToString` _damege))
  (`/Game/Blueprints/BlasterBeam/BP_BlasterBeam.Destroy_BlasterBeam` _asbp_blaster_beam)
  (if (< (`self.HP`) 0)
    (`KismetSystemLibrary.QuitGame` null "Quit")))

(fn `UserConstructionScript`)