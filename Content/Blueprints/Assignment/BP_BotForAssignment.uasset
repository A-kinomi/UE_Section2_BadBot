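; BP_BotForAssignment is a bot actor that chases the assignment's small sphere.
; Each Tick it looks up the BP_AssignemntSmallSphere actor and smoothly rotates toward it using RInterpTo on a look-at rotation.
; It then moves along its forward vector at MoveSpeed scaled by delta time, without sweep, so it passes through collision.
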(event `self.ReceiveTick`
  (params (DeltaSeconds :type "Float (single-precision)"))
  (bind _returnvalue (`GameplayStatics.GetActorOfClass` "/Game/Blueprints/Assignment/BP_AssignemntSmallSphere.BP_AssignemntSmallSphere_C"))
  (set `self.SmallSphere` _returnvalue)
  (`self.K2_SetActorRotation` (`KismetMathLibrary.RInterpTo` (`self.K2_GetActorRotation`) (`KismetMathLibrary.FindLookAtRotation` (`self.K2_GetActorLocation`) (`self.K2_GetActorLocation` (`self.SmallSphere`))) DeltaSeconds 10.0))
  (`self.K2_AddActorWorldOffset` (* (`self.GetActorForwardVector`) (* (`self.MoveSpeed`) (`GameplayStatics.GetWorldDeltaSeconds`)))))

(fn `UserConstructionScript`)