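; Spawner actor for a point-scoring assignment that places small sphere targets and counts hits on them.
; On BeginPlay it draws a temporary debug sphere and spawns a BP_AssignemntSmallSphere, offsetting the actor location by a random point from the Box component's bounds.
; Each sphere's OnBotHit event is bound to IncreasePoint, which increments and prints the score, then spawns the next sphere.
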(event `self.ReceiveBeginPlay`
  (`KismetSystemLibrary.DrawDebugSphere` (0.0 0.0 0.0) (`self.SpawnArea`) 12 (struct :`R` 1.0 :`G` 1.0 :`B` 1.0 :`A` 1.0) 30.0)
  (`self.SpawnSphere`))

(event `SpawnSphere`
  (bind (_origin _boxextent) (`KismetSystemLibrary.GetComponentBounds` (`self.Box`)))
  (bind _returnvalue (`|SpawnActorFromClass` "/Game/Blueprints/Assignment/BP_AssignemntSmallSphere.BP_AssignemntSmallSphere_C" (`KismetMathLibrary.MakeTransform` (+ (`self.K2_GetActorLocation`) (`KismetMathLibrary.RandomPointInBoundingBox` _origin _boxextent))) "Undefined" "MultiplyWithRoot" null false null))
  (add `/Game/Blueprints/Assignment/BP_AssignemntSmallSphere.OnBotHit` _returnvalue (delegate `IncreasePoint`)))

(event `IncreasePoint`
  ;[1 1 1] Count Points
  (bind _output_get (set `self.PointCount` (+ (`self.PointCount`) 1)))
  (`KismetSystemLibrary.PrintString` (`KismetStringLibrary.Concat_StrStr` (`KismetStringLibrary.Conv_IntToString` _output_get) " Point"))
  (`self.SpawnSphere`))

(fn `UserConstructionScript`)